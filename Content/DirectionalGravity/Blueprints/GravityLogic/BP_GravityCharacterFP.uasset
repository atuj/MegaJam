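; First-person player character for a directional-gravity shooter: it flips gravity, fires a hitscan gun and triggers the win and death screens.
; The Ability input alternates the level's gravity volume between upright and rotated 180 degrees; firing line-traces from the muzzle and sends damage through an interface message.
; Tick aligns side collision to the camera, re-creates the crosshair widget every frame and shows victory when no bots remain.
; Lethal damage resets gravity, plays death and briefly possesses a spectator pawn.
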(event `self.ReceiveBeginPlay`
  (bind _returnvalue (`GameplayStatics.GetActorOfClass` "/Game/DirectionalGravity/Blueprints/SceneObjects/BP_GravityVolumeBox.BP_GravityVolumeBox_C"))
  (set `self.GravityVolumeBox` _returnvalue)
  (bind _asbp_game_instance (cast `/Game/MegaJam/Core/Blueprints/BP_GameInstance` (`GameplayStatics.GetGameInstance`)))
  (set `self.As BP Game Instance` _asbp_game_instance))

(event `self.ReceiveTick`
  (params (DeltaSeconds :type "Float (single-precision)"))
  (bind (_returnvalue_roll _returnvalue_pitch _returnvalue_yaw) (`KismetMathLibrary.BreakRotator` (`SceneComponent.K2_GetComponentRotation` (`self.Camera`))))
  (`parent.ReceiveTick` DeltaSeconds)
  (`SceneComponent.K2_SetWorldRotation` (`self.SideCollision`) (`KismetMathLibrary.MakeRotator` _returnvalue_roll _returnvalue_pitch _returnvalue_yaw) false false)
  (bind _returnvalue (`|CreateWidget` "/Game/MegaJam/ThirdPersonBP/TestFloader/cursor.cursor_C" (`GameplayStatics.GetPlayerController` 0)))
  (set `self.WBPCursorCrosshair` _returnvalue)
  (`UserWidget.AddToViewport` (`self.WBPCursorCrosshair`) 0)
  (bind _outactors (`GameplayStatics.GetAllActorsOfClass` "/Game/MegaJam/Core/Bots/Blueprints/BP_BotCharacter.BP_BotCharacter_C"))
  (if (== (`KismetArrayLibrary.Array_Length` _outactors) 0)
    (`/Engine/EditorBlueprintResources/StandardMacros.DoOnce` false
      (:`Completed`
        (`/Game/MegaJam/Core/Blueprints/BP_GameInstance.ShowWinnerScreen` (`self.As BP Game Instance`))))))

(event `InputAction|Ability`
  (params (Key :type "Key Structure"))
  (bind _gravityvolumebox (`self.GravityVolumeBox`))
  (:`Pressed`
    (`|PlayMontage` (`self.SkeletalMesh`) "/Game/MegaJam/ThirdPersonBP/NewAnimation/AM_GravityChange.AM_GravityChange" 10.0
      (:`then`
        (`/Engine/EditorBlueprintResources/StandardMacros.FlipFlop`
          (:`A`
            (`self.K2_SetActorRotation` _gravityvolumebox (struct :`Pitch` 180.0) false))
          (:`B`
            (`self.K2_SetActorRotation` :`self` _gravityvolumebox :!label _label)))))))

(event `Rotate player in base`
  (goto _label))

(event `InputAction|Fire`
  (params (Key :type "Key Structure"))
  (bind (_bblockinghit _binitialoverlap _time _distance _location _impactpoint _normal _impactnormal) (`GameplayStatics.BreakHitResult` (`self.Out Hit`)))
  (bind (_bblockinghit_2 _binitialoverlap_2 _time_2 _distance_2 _location_2 _impactpoint_2 _normal_2 _impactnormal_2 _physmat _hitactor) (`GameplayStatics.BreakHitResult` (`self.Out Hit`)))
  (bind _location_3 (.location (`SceneComponent.GetSocketTransform` (`self.SkeletalMesh`) "SOCKET_Muzzle" "RTS_World")))
  ;[0.125 0 1] Fire
  (:`Pressed`
    (`/Engine/EditorBlueprintResources/StandardMacros.IsValid` (`self.Monage Fire`)
      (:`Is Valid`
        (`GameplayStatics.PlaySoundAtLocation` "/Game/LPSPSample/Audio/SC_WEP_Fire_03.SC_WEP_Fire_03" (`SceneComponent.GetSocketLocation` (`self.SkeletalMesh`) "SOCKET_Muzzle") (struct) 1.0 1.0 0.0 null null null)
        (set `self.Ammunition Current` (`KismetMathLibrary.Clamp` (- (`self.Ammunition Current`) 1) 0 (`self.Ammunition Max`)))
        (`GameplayStatics.SpawnEmitterAttached` "/Game/LPSPSample/Art/Effects/PS_MFlash.PS_MFlash" (`self.SkeletalMesh`) "SOCKET_Muzzle" (0.0 0.0 0.0) (struct :`Yaw` -90.0))
        (bind (_outhit _returnvalue) (`KismetSystemLibrary.LineTraceSingle` :`Start` _location_3 :`End` (+ _location_3 (* (`KismetMathLibrary.Normal` (`KismetMathLibrary.GetForwardVector` (`SceneComponent.K2_GetComponentRotation` (`self.Camera`)))) 10000.0)) :`TraceChannel` "TraceTypeQuery1" :`DrawTime` 1.0))
        (set `self.Out Hit` _outhit)
        (if _returnvalue
          (`GameplayStatics.SpawnDecalAtLocation` "/Game/LPSPSample/Art/Effects/MI_Decal_Bullet_Concrete.MI_Decal_Bullet_Concrete" (5.0 5.0 5.0) _impactpoint (`KismetMathLibrary.Conv_VectorToRotator` _impactnormal) 15.0)
          (`|PlayMontage` (`self.SkeletalMesh`) "/Game/MegaJam/ThirdPersonBP/NewAnimation/AM_FireFinger.AM_FireFinger" 15.0
            (:`then`
              (`GameplayStatics.PlayWorldCameraShake` "/Game/MegaJam/ThirdPersonBP/Blueprints/MyShake.MyShake_C" (`SceneComponent.K2_GetComponentLocation` (`self.Camera`)) 0.0 500.0)
              (`GameplayStatics.SpawnEmitterAtLocation` "/Game/LPSPSample/Art/Effects/PS_Impact.PS_Impact" _impactpoint_2 (`KismetMathLibrary.Conv_VectorToRotator` _impactnormal_2) (0.8 0.8 0.8))
              (`GameplayStatics.SpawnSoundAtLocation` "/Game/LPSPSample/Audio/SC_WEP_Impact_Bullet.SC_WEP_Impact_Bullet" (`.ImpactPoint` (`GameplayStatics.BreakHitResult` (`self.Out Hit`))) (struct) 1.0 1.0 0.0 null null)
              (message `/Game/LPSPSample/Core/BPI_LPSP_Damageable.On Receive Damage Point` (`.HitActor` (`GameplayStatics.BreakHitResult` (`self.Out Hit`))) (`self.Damage`)))))))))

(event `/Game/LPSPSample/Core/BPI_LPSP_Damageable.On Receive Damage Point`
  (params (Damage :type "Float (single-precision)"))
  (bind _returnvalue (`GameplayStatics.GetPlayerController` 0))
  (bind _health (`self.Health`))
  (set `self.Health` (- _health Damage))
  (if (<= _health 0.0) :!label _label_2
    (`/Engine/EditorBlueprintResources/StandardMacros.DoOnce` false
      (:`Completed`
        ;[1 1 1] Comment
        (`self.Rotate player in base`)
        (`KismetSystemLibrary.Delay` 1.5)
        (`PrimitiveComponent.SetCollisionEnabled` (`self.WalkCollision`) "PhysicsOnly")
        (`PrimitiveComponent.SetCollisionEnabled` (`self.SideCollision`) "PhysicsOnly")
        (`SkeletalMeshComponent.PlayAnimation` (`self.SkeletalMesh`) "/Game/AnimStarterPack/Death_1.Death_1" false)
        ;[1 1 1] Comment
        (bind _returnvalue_2 (`|SpawnActorFromClass` "/Script/Engine.SpectatorPawn" (`self.GetTransform`) "Undefined" "OverrideRootScale" null null))
        (`Controller.Possess` _returnvalue _returnvalue_2)
        (`KismetSystemLibrary.Delay` 3.0)
        (`Controller.UnPossess` _returnvalue)
        ;[1 1 1] Comment
        (`/Game/MegaJam/Core/Blueprints/BP_GameInstance.ShowDeadScreen` (`self.As BP Game Instance`))))))

(event `/Game/LPSPSample/Core/BPI_LPSP_Damageable.On Receive Damage Radial`
  (set `self.Health` (- (`self.Health`) 50.0))
  (goto _label_2))

(fn `GetCharacterSpeed`
  (returns (Cspeed :type "Float (double-precision)"))
  (return (`KismetMathLibrary.VSize` (`SceneComponent.GetComponentVelocity` (`self.WalkCollision`)))))

(fn `GetEnemy`
  (returns (CountEnemy :type Integer))
  (bind _outactors (`GameplayStatics.GetAllActorsOfClass` "/Game/MegaJam/Core/Bots/Blueprints/BP_BotCharacter.BP_BotCharacter_C"))
  (return (`KismetArrayLibrary.Array_Length` _outactors)))

(fn `GetRotation`
  (returns (NewRotation :type "Float (double-precision)"))
  (bind (_returnvalue_roll _returnvalue_pitch) (`KismetMathLibrary.BreakRotator` (`SceneComponent.K2_GetComponentRotation` (`self.Camera`))))
  (return _returnvalue_pitch))

(fn `IsPlayer`
  (returns (IsPLayer :type Boolean))
  (return true))

(fn `UserConstructionScript`
  (`parent.UserConstructionScript`))