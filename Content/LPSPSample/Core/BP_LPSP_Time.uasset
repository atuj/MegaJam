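; BP_LPSP_Time is a debug-style time controller that lets the player slow, speed up or pause game time.
; Speed-up and slow-down actions and a time axis step the target scale by a set increment, clamped between zero and one.
; Tick smoothly interpolates global time dilation toward that target.
; A hard-wired 5 key toggles game pause through a flip-flop.
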(event `self.ReceiveBeginPlay`
  ;[0.3125 0 1] Begin Play
  (`parent.ReceiveBeginPlay`)
  (set `self.Time Scale Current` (`self.Time Scale Default`)))

(event `self.ReceiveTick`
  (params (DeltaSeconds :type "Float (single-precision)"))
  ;[0.125 0 1] Tick
  (`parent.ReceiveTick` DeltaSeconds)
  (`GameplayStatics.SetGlobalTimeDilation` (`KismetMathLibrary.FInterpTo` (`GameplayStatics.GetGlobalTimeDilation`) (`self.Time Scale Current`) DeltaSeconds 20.0)))

(event `InputAction|Time (Speed Up)`
  (params (Key :type "Key Structure"))
  ;[1 0 0.6562] Increase
  (:`Pressed`
    (`self.Update Time Scale` (+ (`self.Time Scale Current`) (`self.Time Scale Increments`)))))

(event `InputAction|Time (Slow Down)`
  (params (Key :type "Key Structure"))
  ;[0.6641 0 1] Decrease
  (:`Pressed`
    (`self.Update Time Scale` (- (`self.Time Scale Current`) (`self.Time Scale Increments`)))))

(event `InputAxis|Time` :consume false
  (params (AxisValue :type "Float (single-precision)"))
  ;[0 1 0.2969] Time Axis
  (`self.Update Time Scale` (+ (* AxisValue (`self.Time Scale Increments`)) (`self.Time Scale Current`))))

(event `Key|Five` :paused true
  (params (Key :type "Key Structure"))
  ;[1 0 0.6094] Stop
  (:`Pressed`
    (`/Engine/EditorBlueprintResources/StandardMacros.FlipFlop`
      (:`A`
        (`GameplayStatics.SetGamePaused` true))
      (:`B`
        (`GameplayStatics.SetGamePaused` false)))))

(fn `Update Time Scale`
  (params (Value :type "Float (double-precision)"))
  (bind _returnvalue (`KismetMathLibrary.FClamp` Value))
  (`|ExecutionSequence`
    (:`then_0`
      (if (not (== (`self.Time Scale Current`) _returnvalue))
        (set `self.Time Scale Current` _returnvalue)))
    (:`then_1`
      (return))))

(fn `UserConstructionScript`)