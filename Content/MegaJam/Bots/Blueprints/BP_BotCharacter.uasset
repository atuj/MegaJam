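; AI bot character that carries a rifle, spawned on BeginPlay and attached to the Gun socket.
; OnStartFire shoots once per loop step through the current ammo, reloads with montages, then restarts after a pause; OnEndFire breaks the loop.
; CheckDistancePlayer moves the bot to an EQS-chosen location.
; Getters expose the controller's target, the aiming flag and a scaled vertical pitch toward the player.
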(event `self.ReceiveBeginPlay`
  ;[1 1 1] Begin Play
  (bind _returnvalue (`|SpawnActorFromClass` "/Game/LPSPSample/Useable/Weapons/BP_LPSP_WEP_Rifle.BP_LPSP_WEP_Rifle_C" (`KismetMathLibrary.MakeTransform` (0.0 0.0 0.0)) "Undefined" "OverrideRootScale" self self))
  (bind _output_get (set `self.Weapon` _returnvalue))
  (`self.K2_AttachToComponent` _output_get (`self.Mesh`) "Gun" "KeepRelative" "KeepRelative" "KeepRelative" true))

(event `self.OnStartFire`
  (bind _returnvalue (message `/Game/LPSPSample/Core/BPI_LPSP_WEP.Get Ammunition Current` (`self.Weapon`)))
  (`/Game/MegaJam/Blueprints/BPML_BaseMacroLibrari.LoopWithBreakWithDelay` 1 _returnvalue 1.0 :!label _label
    (:`LoopBody`
      (message `/Game/LPSPSample/Core/BPI_LPSP_WEP.On Fire` (`self.Weapon`))
      (`|PlayMontage` (`self.Mesh`) "/Game/MegaJam/ThirdPersonBP/NewAnimation/AM_FireRifle.AM_FireRifle"))
    (:`Completed`
      (message `/Game/LPSPSample/Core/BPI_LPSP_WEP.On Reload` (`self.Weapon`))
      (`|PlayMontage` (`self.Mesh`) "/Game/MegaJam/ThirdPersonBP/NewAnimation/AM_RifleReloadAim.AM_RifleReloadAim"
        (:`OnCompleted`
          (`KismetSystemLibrary.Delay` 3.0)
          (`self.OnStartFire`))))))

(event `self.OnEndFire`
  (goto _label :!via `Break`))

(event `self.SetAiming`
  (params (`Set?` :type Boolean))
  (set `self.Aiming` `Set?`))

(event `self.CheckDistancePlayer`
  (bind _returnvalue (`EnvQueryManager.RunEQSQuery` "/Game/MegaJam/Bots/EQS/EQS_CheckDistanceTOPLayer.EQS_CheckDistanceTOPLayer" self "SingleResult"))
  (`KismetSystemLibrary.Delay` (`GameplayStatics.GetWorldDeltaSeconds`))
  (bind (_resultlocations _returnvalue_2) (`EnvQueryInstanceBlueprintWrapper.GetQueryResultsAsLocations` _returnvalue))
  (if _returnvalue_2
    (`|AIMoveTo` self (`|GetArrayItem` _resultlocations) null)))

(fn `GetTargetActor`
  (returns (Actor :type "Actor Object Reference"))
  (bind _actor (message `/Game/MegaJam/Bots/Blueprints/BPI_Bots.GetTargetActor` (`self.GetController`)))
  (return _actor))

(fn `GetUpRotation`
  (returns (UpDegrees :type "Float (double-precision)"))
  (bind (_returnvalue_x _returnvalue_y _returnvalue_z) (`KismetMathLibrary.BreakVector` (`self.K2_GetActorLocation`)))
  (bind _ashero_character (cast `/Game/MegaJam/ThirdPersonBP/NewAnimation/HeroCharacter` (`GameplayStatics.GetPlayerCharacter` 0)))
  (bind (_returnvalue_x_2 _returnvalue_y_2) (`KismetMathLibrary.BreakVector` (`self.K2_GetActorLocation` _ashero_character)))
  (bind (_returnvalue_roll _returnvalue_pitch) (`KismetMathLibrary.BreakRotator` (`KismetMathLibrary.NormalizedDeltaRotator` (`KismetMathLibrary.FindLookAtRotation` (`KismetMathLibrary.MakeVector` _returnvalue_x _returnvalue_y _returnvalue_z) (`KismetMathLibrary.MakeVector` _returnvalue_x_2 _returnvalue_y_2 _returnvalue_z)) (`KismetMathLibrary.FindLookAtRotation` (`self.K2_GetActorLocation`) (`self.K2_GetActorLocation` _ashero_character)))))
  (return (* _returnvalue_pitch -1.5)))

(fn `IsAiming`
  (returns (IsAiming :type Boolean))
  (return (`self.Aiming`)))

(fn `UserConstructionScript`)