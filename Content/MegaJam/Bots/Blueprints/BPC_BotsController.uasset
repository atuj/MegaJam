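; AI controller for bots that detects the player through AI perception and drives the possessed pawn's aim and fire.
; On sensing the player it stores the target, focuses on it, starts aiming and firing, and runs a looping timer that asks the pawn to check player distance.
; Losing the player clears target and focus and stops fire, but not the timer.
; It exposes the target, while up-rotation and aiming getters return fixed defaults.
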(event `self.AIPerception.OnTargetPerceptionUpdated`
  (params (Actor :type "Actor Object Reference") (Stimulus :type "AIStimulus Structure"))
  (bind _returnvalue (`self.K2_GetPawn`))
  (bind _returnvalue_2 (`self.K2_GetPawn`))
  (bind _isplayer (message `/Game/MegaJam/ThirdPersonBP/Blueprints/BPI_PlayerCharacter.IsPlayer` Actor))
  (if _isplayer
    (if (`.bSuccessfullySensed` (break `AIStimulus` Stimulus))
      (set `self.ActorTarget` Actor)
      (`KismetSystemLibrary.K2_SetTimer` null "CheckDistance" 1.0 true)
      (message `/Game/MegaJam/Bots/Blueprints/BPI_Bots.SetAiming` _returnvalue_2 true)
      (`self.K2_SetFocus` (`self.ActorTarget`))
      (message `/Game/MegaJam/Bots/Blueprints/BPI_Bots.OnStartFire` _returnvalue)
      (else
        (set `self.ActorTarget` null)
        (message `/Game/MegaJam/Bots/Blueprints/BPI_Bots.SetAiming` _returnvalue_2 false)
        (`self.K2_ClearFocus`)
        (message `/Game/MegaJam/Bots/Blueprints/BPI_Bots.OnEndFire` _returnvalue)))))

(fn `CheckDistance`
  (message `/Game/MegaJam/Bots/Blueprints/BPI_Bots.CheckDistancePlayer` (`self.K2_GetPawn`)))

(fn `GetTargetActor`
  (returns (Actor :type "Actor Object Reference"))
  (return (`self.ActorTarget`)))

(fn `GetUpRotation`
  (returns (UpDegrees :type "Float (double-precision)"))
  (return 0.0))

(fn `IsAiming`
  (returns (IsAiming :type Boolean))
  (return false))

(fn `UserConstructionScript`)