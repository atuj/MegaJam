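; AI controller for bots that spots the player and drives the controlled pawn's aiming and firing.
; AI Perception updates on player actors set the target and focus while sensed and the bot has health, sending fire and aim interface messages to the pawn.
; Otherwise, or on EraseBotsStates, it clears target and focus and stops firing.
; GetTargetActor exposes the target; GetUpRotation and IsAiming return fixed stub values.
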(event `self.AIPerception.OnTargetPerceptionUpdated`
  (params (Actor :type "Actor Object Reference") (Stimulus :type "AIStimulus Structure"))
  (bind _returnvalue (`self.K2_GetPawn`))
  (bind _returnvalue_2 (`self.K2_GetPawn`))
  (bind _returnvalue_3 (`self.K2_GetPawn`))
  (bind _isplayer (message `/Game/MegaJam/ThirdPersonBP/Blueprints/BPI_PlayerCharacter.IsPlayer` Actor))
  (if _isplayer
    (if (and (`.bSuccessfullySensed` (break `AIStimulus` Stimulus)) (> (`/Game/MegaJam/Core/Bots/Blueprints/BP_BotCharacter.Health` (cast `/Game/MegaJam/Core/Bots/Blueprints/BP_BotCharacter` (`self.K2_GetPawn`) :!pure true)) 0.0))
      (set `self.ActorTarget` Actor)
      (`KismetSystemLibrary.PrintString` "view")
      (message `/Game/MegaJam/Core/Bots/Blueprints/BPI_Bots.OnStartFire` _returnvalue_3)
      (message `/Game/MegaJam/Core/Bots/Blueprints/BPI_Bots.SetAiming` _returnvalue_2 true)
      (`self.K2_SetFocus` (`self.ActorTarget`))
      (message `/Game/MegaJam/Core/Bots/Blueprints/BPI_Bots.OnStartFire` _returnvalue)
      (else
        (set `self.ActorTarget` null :!label _label)
        (message `/Game/MegaJam/Core/Bots/Blueprints/BPI_Bots.OnEndFire` _returnvalue_3)
        (message `/Game/MegaJam/Core/Bots/Blueprints/BPI_Bots.SetAiming` _returnvalue_2 false)
        (`self.K2_ClearFocus`)
        (message `/Game/MegaJam/Core/Bots/Blueprints/BPI_Bots.OnEndFire` _returnvalue)))))

(event `EraseBotsStates`
  (goto _label))

(fn `GetTargetActor`
  (returns (Actor :type "Actor Object Reference"))
  (return (`self.ActorTarget`)))

(fn `GetUpRotation`
  (returns (UpDegrees :type "Float (double-precision)"))
  (return 0.0))

(fn `IsAiming`
  (returns (IsAiming :type Boolean))
  (return false))

(fn `UserConstructionScript`)