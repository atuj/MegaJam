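; Enemy bot character that fights with a rifle spawned on its Gun socket and works with BPC_BotsController.
; Firing runs random bursts, reloads when empty, then non-sniper bots move to an EQS-picked point and resume firing.
; Point and radial damage reduce health; death reports the kill to the player, clears controller state and perception, plays a random animation, then sinks and destroys the body.
; GetUpRotation derives vertical aim pitch toward the player.
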(event `self.ReceiveBeginPlay`
  ;[1 1 1] Begin Play
  (bind _asbpc_bots_controller (cast `/Game/MegaJam/Core/Bots/Blueprints/BPC_BotsController` (`self.GetController`)))
  (set `self.BPCBotsController` _asbpc_bots_controller)
  (bind _returnvalue (`|SpawnActorFromClass` "/Game/LPSPSample/Useable/Weapons/BP_LPSP_WEP_Rifle.BP_LPSP_WEP_Rifle_C" (`KismetMathLibrary.MakeTransform` (0.0 0.0 0.0)) "Undefined" "OverrideRootScale" self self))
  (bind _output_get (set `self.Weapon` _returnvalue))
  (`self.K2_AttachToComponent` _output_get (`self.Mesh`) "Gun" "KeepRelative" "KeepRelative" "KeepRelative" true))

(event `self.OnStartFire`
  (bind _returnvalue (message `/Game/LPSPSample/Core/BPI_LPSP_WEP.Get Ammunition Current` (`self.Weapon`)))
  (if (!= _returnvalue 0)
    (`/Game/MegaJam/Core/Blueprints/BPML_BaseMacroLibrari.LoopWithBreakWithDelay` 1 (`KismetMathLibrary.RandomInteger` 10) (`KismetMathLibrary.RandomFloat`) :!label _label
      (:`LoopBody`
        (message `/Game/LPSPSample/Core/BPI_LPSP_WEP.On Fire` (`self.Weapon`))
        (`|PlayMontage` (`self.Mesh`) "/Game/MegaJam/ThirdPersonBP/NewAnimation/AM_FireRifle.AM_FireRifle"))
      (:`Completed`
        (`self.CheckDistancePlayer`)))
    (else
      (`MovementComponent.StopMovementImmediately` (`self.CharacterMovement`))
      (set `self.IsReload` true)
      (message `/Game/LPSPSample/Core/BPI_LPSP_WEP.On Reload` (`self.Weapon`))
      (`|PlayMontage` (`self.Mesh`) "/Game/MegaJam/ThirdPersonBP/NewAnimation/AM_RifleReloadAim.AM_RifleReloadAim" 1.1
        (:`OnCompleted`
          (`KismetSystemLibrary.Delay` 3.0)
          (set `self.IsReload` false)
          (`self.OnStartFire`))))))

(event `self.OnEndFire`
  (goto _label :!via `Break`))

(event `/Game/LPSPSample/Core/BPI_LPSP_Damageable.On Receive Damage Point`
  (params (Damage :type "Float (single-precision)"))
  (bind _health (`self.Health`))
  (bind _mesh (`self.Mesh`))
  (bind _capsulecomponent (`self.CapsuleComponent`))
  (bind (_returnvalue_x _returnvalue_y _returnvalue_z) (`KismetMathLibrary.BreakVector` (`SceneComponent.K2_GetComponentLocation` _capsulecomponent)))
  (set `self.Health` (- _health Damage))
  (if (<= _health 0.0) :!label _label_2
    (`/Engine/EditorBlueprintResources/StandardMacros.DoOnce` false
      (:`Completed`
        (message `/Game/MegaJam/ThirdPersonBP/Blueprints/BPI_PlayerCharacter.MakeKill` (`GameplayStatics.GetPlayerPawn` 0))
        (`/Game/MegaJam/Core/Bots/Blueprints/BPC_BotsController.EraseBotsStates` (`self.BPCBotsController`))
        (`CharacterMovementComponent.DisableMovement` (`self.CharacterMovement`))
        (`PrimitiveComponent.SetCollisionEnabled` (`self.CapsuleComponent`) "NoCollision")
        (switch `int` (`KismetMathLibrary.Round` (`KismetMathLibrary.RandomFloatInRange` 0.0 4.0))
          (:`0`
            (`SkeletalMeshComponent.PlayAnimation` _mesh "/Game/AnimStarterPack/Death_Ironsights_1.Death_Ironsights_1" false))
          (:`1`
            (`SkeletalMeshComponent.PlayAnimation` _mesh "/Game/AnimStarterPack/Death_Ironsights_2.Death_Ironsights_2" false))
          (:`2`
            (`SkeletalMeshComponent.PlayAnimation` _mesh "/Game/AnimStarterPack/Death_1.Death_1" false))
          (:`3`
            (`SkeletalMeshComponent.PlayAnimation` _mesh "/Game/AnimStarterPack/Death_2.Death_2" false)))
        (`ActorComponent.K2_DestroyComponent` (`/Game/MegaJam/Core/Bots/Blueprints/BPC_BotsController.AIPerception` (`self.BPCBotsController`)))
        (`KismetSystemLibrary.Delay` 5.0)
        (`KismetSystemLibrary.MoveComponentTo` _capsulecomponent (`KismetMathLibrary.MakeVector` _returnvalue_x _returnvalue_y (- _returnvalue_z 100.0)) (struct) true true 1.0)
        (`self.K2_DestroyActor`)))))

(event `/Game/LPSPSample/Core/BPI_LPSP_Damageable.On Receive Damage Radial`
  (set `self.Health` (- (`self.Health`) 50.0))
  (goto _label_2))

(event `self.SetAiming`
  (params (`Set?` :type Boolean))
  (set `self.Aiming` `Set?`))

(event `CheckDistancePlayer`
  (if (not (`self.Sniper`))
    (bind _returnvalue (`EnvQueryManager.RunEQSQuery` "/Game/MegaJam/Core/Bots/EQS/EQS_CheckDistanceTOPLayer.EQS_CheckDistanceTOPLayer" self "SingleResult"))
    (`KismetSystemLibrary.Delay` (`GameplayStatics.GetWorldDeltaSeconds`))
    (bind (_resultlocations _returnvalue_2) (`EnvQueryInstanceBlueprintWrapper.GetQueryResultsAsLocations` _returnvalue))
    (if _returnvalue_2
      (`|AIMoveTo` self (`|GetArrayItem` _resultlocations) null 50.0
        (:`OnSuccess`
          _)
        (:`OnFail`
          _))
      (`self.OnStartFire`))))

(fn `GetHealth`
  (returns (CurrentHealth :type "Float (double-precision)"))
  (return (`self.Health`)))

(fn `GetTargetActor`
  (returns (Actor :type "Actor Object Reference"))
  (bind _actor (message `/Game/MegaJam/Core/Bots/Blueprints/BPI_Bots.GetTargetActor` (`self.GetController`)))
  (return _actor))

(fn `GetUpRotation`
  (returns (UpDegrees :type "Float (double-precision)"))
  (bind (_returnvalue_x _returnvalue_y _returnvalue_z) (`KismetMathLibrary.BreakVector` (`self.K2_GetActorLocation`)))
  (bind _asbp_gravity_character_fp (cast `/Game/DirectionalGravity/Blueprints/GravityLogic/BP_GravityCharacterFP` (`GameplayStatics.GetPlayerPawn` 0)))
  (bind (_returnvalue_x_2 _returnvalue_y_2) (`KismetMathLibrary.BreakVector` (`self.K2_GetActorLocation` _asbp_gravity_character_fp)))
  (bind (_returnvalue_roll _returnvalue_pitch) (`KismetMathLibrary.BreakRotator` (`KismetMathLibrary.NormalizedDeltaRotator` (`KismetMathLibrary.FindLookAtRotation` (`KismetMathLibrary.MakeVector` _returnvalue_x _returnvalue_y _returnvalue_z) (`KismetMathLibrary.MakeVector` _returnvalue_x_2 _returnvalue_y_2 _returnvalue_z)) (`KismetMathLibrary.FindLookAtRotation` (`self.K2_GetActorLocation`) (`self.K2_GetActorLocation` _asbp_gravity_character_fp)))))
  (return (* _returnvalue_pitch -1.5)))

(fn `IsAiming`
  (returns (IsAiming :type Boolean))
  (return (`self.Aiming`)))

(fn `UserConstructionScript`)